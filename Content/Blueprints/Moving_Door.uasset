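; Template sliding door actor that players open and close with the Interact input while inside its trigger box.
; Overlap enables input and shows a Keypad_Widget prompt with the bound key and open/close wording; leaving hides it and disables input.
; The construction script derives the end position from an Axis Motion offset.
; Two timelines lerp the placeholder mesh between endpoints, with a Playing flag blocking input mid-move.
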(event `self.Trigger.OnComponentBeginOverlap`
  (params (OverlappedComponent :type "PrimitiveComponent Object Reference") (OtherActor :type "Actor Object Reference") (OtherComp :type "PrimitiveComponent Object Reference") (OtherBodyIndex :type Integer) (bFromSweep :type Boolean) (SweepResult :type "HitResult Structure (by ref)"))
  ;[1 1 1] This block here enables input whenever a player enters a trigger box. It sets the text that gets displayed when you walk up to the interaction box, including getting the key you set for the Interact button (in project settings)
  (`self.EnableInput` (`GameplayStatics.GetPlayerController` 0))
  (bind _askeypad_widget (cast `/Game/Blueprints/Keypad_Widget` (`WidgetComponent.GetUserWidgetObject` (`self.TextWidget`))))
  (if (`self.DoorOpen`)
    (set `/Game/Blueprints/Keypad_Widget.OpenClose` "close" _askeypad_widget)
    (else
      (set `/Game/Blueprints/Keypad_Widget.OpenClose` "open" _askeypad_widget)))
  (`/Game/Blueprints/Keypad_Widget.ShowHideText` _askeypad_widget (`.Key` (break `InputActionKeyMapping` (`|GetArrayItem` (`InputSettings.GetActionMappingByName` (`InputSettings.GetInputSettings`) "Interact"))))))

(event `self.Trigger.OnComponentEndOverlap`
  (params (OverlappedComponent :type "PrimitiveComponent Object Reference") (OtherActor :type "Actor Object Reference") (OtherComp :type "PrimitiveComponent Object Reference") (OtherBodyIndex :type Integer))
  ;[1 1 1] This block here enables input whenever a player enters a trigger box. It sets the text that gets displayed when you walk up to the interaction box, including getting the key you set for the Interact button (in project settings)
  (`self.DisableInput` (`GameplayStatics.GetPlayerController` 0))
  (bind _askeypad_widget (cast `/Game/Blueprints/Keypad_Widget` (`WidgetComponent.GetUserWidgetObject` (`self.TextWidget`))))
  (`/Game/Blueprints/Keypad_Widget.HideText` _askeypad_widget))

(event `InputAction|Interact`
  (params (Key :type "Key Structure"))
  (bind _doorbegin (`self.DoorBegin`))
  (bind _doorend (`self.DoorEnd`))
  ;[1 1 1] This handles the input which causes the doors to open and close. Both timelines are identical, but separated in case of ghosting bugs. Make sure to replace the references to the Cube to whichever door you prefer to use. The rest should be taken care of
  (:`Pressed`
    (if (`self.Playing`)
      _
      (elif (`self.DoorOpen`)
        (set `self.DoorOpen` false)
        (bind (_direction _driver) (`Timeline|DoorDriver` :!via `PlayFromStart`)
          (:`Update`
            (`SceneComponent.K2_SetRelativeLocation` (`self.Cube(Replace_this_with_Static_Mesh)`) (`KismetMathLibrary.VLerp` _doorend _doorbegin _driver) false false)
            (set `self.Playing` true)
            (cast `/Game/Blueprints/Keypad_Widget` (`WidgetComponent.GetUserWidgetObject` (`self.TextWidget`)) :!label _label))
          (:`Finished`
            (set `self.Playing` false)))
        (else
          (set `self.DoorOpen` true)
          (bind (_direction_2 _driver_2) (`Timeline|DoorDriver_2` :!via `PlayFromStart`)
            (:`Update`
              (`SceneComponent.K2_SetRelativeLocation` (`self.Cube(Replace_this_with_Static_Mesh)`) (`KismetMathLibrary.VLerp` _doorbegin _doorend _driver_2) false false)
              (set `self.Playing` true)
              (goto _label))
            (:`Finished`
              (set `self.Playing` false))))))))

(fn `UserConstructionScript`
  ;[1 1 1] This sets the initial and end spot for the door. The only variable you can change is the Axis Motion (Which direction do you want it to move, and how much?
  (bind _output_get (set `self.DoorBegin` (`SceneComponent.RelativeLocation` (`self.Cube(Replace_this_with_Static_Mesh)`))))
  (set `self.DoorEnd` (+ _output_get (`self.AxisMotion`))))